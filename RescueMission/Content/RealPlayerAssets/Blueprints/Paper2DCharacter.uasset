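; Player character for a 2D Paper2D side-scroller with running, double jump, shooting and health.
; Tick swaps sprite flipbooks from movement and shooting state, and yaws the controller to face left or right.
; Left mouse fires bullets on a looping timer from a scene component, unless jumping.
; BeginPlay adds a healthbar widget; damage reduces clamped health, death only prints a message, and H applies test damage.
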(event Custom|Handle%20Animation
  (bind _sprite (Variables|Default|GetSprite))
  (bind _charactermovement (Variables|Character|GetCharacterMovement))
  ;[1 1 1] Handle Animation
  (if (AI|Components|NavMovement|IsFalling _charactermovement)
    (Sprite|SetFlipbook (Variables|Default|GetSprite) (select (< (.z (Transformation|GetVelocity)) 0.0) "/Game/RealPlayerAssets/Jump/playerJumpFlipbook.playerJumpFlipbook" "/Game/RealPlayerAssets/Jump/playerJumpFlipbook.playerJumpFlipbook"))
    (elif (> (Math|Vector|VectorLength (Variables|/Script/Engine.MovementComponent|GetVelocity _charactermovement)) 0.0)
      (if (Variables|Bullet|GetisShooting)
        (Sprite|SetFlipbook _sprite "/Game/RealPlayerAssets/RunShoot/RunShootFlipbook.RunShootFlipbook")
        (else
          (Sprite|SetFlipbook _sprite "/Game/RealPlayerAssets/Run/playerRunFlipbook.playerRunFlipbook")))
      (elif (Variables|Bullet|GetisShooting)
        (Sprite|SetFlipbook _sprite "/Game/RealPlayerAssets/Stand/playerStandFlipbook.playerStandFlipbook")
        (else
          (Sprite|SetFlipbook _sprite "/Game/RealPlayerAssets/Stand/playerStandFlipbook.playerStandFlipbook"))))))

(event Custom|Handle%20Rotation
  ;[1 1 1] change rotation depending on the direction you are facing
  (Math|Float|CompareFloat (.x (Variables|/Script/Engine.MovementComponent|GetVelocity (Variables|Character|GetCharacterMovement))) 0.0
    (:>
      (Pawn|SetControlRotation (Pawn|GetController) (Math|Rotator|MakeRotator 0.0 0.0 0.0) :!label _label))
    (:==
      (if (Variables|Default|GetisMovingRight)
        (goto _label)
        (else
          (Pawn|SetControlRotation (Pawn|GetController) (Math|Rotator|MakeRotator 0.0 0.0 1.8e+02) :!label _label_2))))
    (:<
      (goto _label_2))))

(event Custom|Spawn%20Bullets
  ;[1 1 1] firing bullet every 0.3 seconds when left mouse is pressed
  ;;[1 1 1] spawns bullet
  (Game|SpawnActorfromClass "/Game/Bullet/shot/Bullet_BP.Bullet_BP_C" (Transformation|GetWorldTransform (Variables|Default|GetScene)) "Undefined" 0 0))

(event EventBeginPlay
  (bind _returnvalue (UserInterface|CreateWidget "/Game/UIAssets/Widgets/HealthbarWidget.HealthbarWidget_C"))
  (UserInterface|Viewport|AddtoViewport _returnvalue 0))

(event Collision|EventActorBeginOverlap
  (params (OtherActor :type Actor%20Object%20Reference)))

(event EventTick
  (params (DeltaSeconds :type Float%20%28single-precision%29))
  (CallFunction|HandleAnimation)
  (CallFunction|HandleRotation))

(event Game|Damage|EventAnyDamage
  (params (Damage :type Float%20%28single-precision%29) (DamageType :type Damage%20Type%20Object%20Reference) (InstigatedBy :type Controller%20Object%20Reference) (DamageCauser :type Actor%20Object%20Reference))
  ;[1 1 1] Player Taking Damage
  (Variables|Default|SetHealth (Math|Float|Clamp(Float) (- (Variables|Default|GetHealth) Damage) 0.0 (Variables|Default|GetDefault%20Health)))
  (if (and (<= (Variables|Default|GetHealth) 0.0) (not (Variables|Default|GetIs%20Dead)))
    (Variables|Default|SetIs%20Dead true)
    (CallFunction|PlayerDeath)))

(event EventOnLanded
  (params (Hit :type Hit%20Result%20Structure%20%28by%20ref%29))
  ;[1 1 1] Jumping
  (Variables|Default|SetjumpCount 0)
  (Variables|Default|SetisJumping false))

(event Input|ActionEvents|InputActionJump
  (params (Key :type Key%20Structure :default "None"))
  ;[1 1 1] Jumping
  (:Pressed
    (if (== (Variables|Default|GetjumpCount) 0)
      (Character|Jump)
      (Variables|Default|SetisJumping true)
      (Math|Integer|IncrementInt (Variables|Default|GetjumpCount))
      (elif (<= (Variables|Default|GetjumpCount) 1)
        (Character|LaunchCharacter (Math|Vector|MakeVector 0.0 0.0 4e+02) false false)
        (Math|Integer|IncrementInt (Variables|Default|GetjumpCount))
        (else
          (Character|StopJumping)))))
  (:Released
    (Character|StopJumping)))

(event Input|AxisEvents|InputAxisMovement
  (params (AxisValue :type Float%20%28single-precision%29))
  ;[1 1 1] Movement
  (Pawn|Input|AddMovementInput "1.000000, 0,0.000000" AxisValue false)
  ;;[1 1 1] Set the Movement Direction According to Axis
  (if (> AxisValue 0.0)
    (Variables|Default|SetisMovingRight true)
    (elif (< AxisValue 0.0)
      (Variables|Default|SetisMovingRight false))))

(event Input|MouseEvents|LeftMouseButton
  (params (Key :type Key%20Structure :default "None"))
  ;[1 1 1] firing bullet every 0.3 seconds when left mouse is pressed
  (:Pressed
    (if (Variables|Default|GetisJumping)
      (Variables|Bullet|SetisShooting false :!label _label)
      (Utilities|Time|ClearandInvalidateTimerbyHandle (Variables|bullet|GetfireBulletEvent))
      (else
        (Variables|Bullet|SetisShooting true)
        (bind _returnvalue (Utilities|Time|SetTimerbyEvent (delegate Custom|Spawn%20Bullets) (Variables|bullet|GetfireRate) true))
        (Variables|bullet|SetfireBulletEvent _returnvalue)
        ;;[1 1 1] spawns bullet
        (Game|SpawnActorfromClass "/Game/Bullet/shot/Bullet_BP.Bullet_BP_C" (Transformation|GetWorldTransform (Variables|Default|GetScene)) "Undefined" 0 0))))
  (:Released
    (goto _label)))

(event Input|KeyboardEvents|H
  (params (Key :type Key%20Structure :default "None"))
  ;[1 1 1] Damage yeme testi
  (:Pressed
    (Game|Damage|ApplyDamage self 2e+01 0 0)))

(fn ConstructionScript
  (Variables|Default|SetHealth (Variables|Default|GetDefault%20Health)))

(fn PlayerDeath
  (Development|PrintString "I DIED THE END"))