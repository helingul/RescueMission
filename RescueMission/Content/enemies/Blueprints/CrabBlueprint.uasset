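; Crab enemy pawn that walks sideways along the world X axis.
; BeginPlay picks left or right at random, and Tick feeds constant movement input in that direction.
; Nothing in this graph changes direction afterward, and a sprite X-scale flip based on direction exists but is unconnected, so it never runs.
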(event EventTick
  (params (DeltaSeconds :type Float%20%28single-precision%29))
  (Pawn|Input|AddMovementInput "1.000000, 0, 0" (select (Variables|Default|GetisMovingRight) 1.0 -1.0) false))

(event EventBeginPlay
  (Variables|Default|SetisMovingRight (Math|Random|RandomBool)))

(fn ConstructionScript
  (|CallParentFunction))